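; BP_Pawn is a player-controlled aircraft pawn that constantly moves forward and fires rockets.
; BeginPlay adds the Enhanced Input mapping context, while legacy Pitch and Roll axis events feed controller rotation input.
; Tick applies forward movement input and spins both propellers by delta time, each using a different speed variable.
; The IA_Fire Enhanced Input action spawns BP_Rocket at the Arrow component's transform.
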(event `InputAxis|Roll`
  (params (AxisValue :type "Float (single-precision)"))
  (`self.AddControllerRollInput` AxisValue))

(event `self.ReceiveBeginPlay`
  (`/Engine/EditorBlueprintResources/StandardMacros.IsValid` (`GameplayStatics.GetPlayerController` 0)
    (:`Is Valid`
      (`EnhancedInputSubsystemInterface.AddMappingContext` (pcsubsystem `EnhancedInputLocalPlayerSubsystem` (`GameplayStatics.GetPlayerController` 0)) "/Game/Blueprints/IMC_Input.IMC_Input" 0 (struct)))))

(event `InputAxis|Pitch`
  (params (AxisValue :type "Float (single-precision)"))
  (`self.AddControllerPitchInput` AxisValue))

(event `InputAction|Fire`
  (params (Key :type "Key Structure"))
  ;[1 1 1] Fire Rocket
)

(event `self.ReceiveTick`
  (params (DeltaSeconds :type "Float (single-precision)"))
  ;[1 1 1] Forward 방향으로 움직여라
  (`self.AddMovementInput` (`self.GetActorForwardVector`))
  ;[1 1 1] Right Propeller
  (`SceneComponent.K2_AddLocalRotation` (`self.Right`) (`KismetMathLibrary.MakeRotator` (* (`GameplayStatics.GetWorldDeltaSeconds`) (`self.Time`))) false false)
  ;[1 1 1] Left Propeller
  (`SceneComponent.K2_AddLocalRotation` (`self.Left`) (* (`self.PropellerRotateSpeed`) (`GameplayStatics.GetWorldDeltaSeconds`)) false false))

(event `EnhancedInput|/Game/Blueprints/IA_Fire`
  (params (ActionValue :type Boolean) (ElapsedSeconds :type "Float (double-precision)") (TriggeredSeconds :type "Float (double-precision)") (InputAction :type "InputAction Object Reference" :default "/Game/Blueprints/IA_Fire.IA_Fire"))
  ;[1 1 1] Fire Rocket
  (:`Triggered`
    (`|SpawnActorFromClass` "/Game/Maps/BP_Rocket.BP_Rocket_C" (`SceneComponent.K2_GetComponentToWorld` (`self.Arrow`)) "Undefined" "OverrideRootScale" null null)))

(fn `UserConstructionScript`)