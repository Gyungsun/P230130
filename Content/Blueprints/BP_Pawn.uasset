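; BP_Pawn is a pawn with spinning left and right propellers, steered through controller rotation input.
; The Forward axis feeds controller roll and the Side axis feeds controller pitch.
; Every tick, both propeller components rotate around their local X (roll) axis by world delta seconds times the Time variable, which acts as a frame-rate-independent spin speed.
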(event `InputAxis|Forward`
  (params (AxisValue :type "Float (single-precision)"))
  (`self.AddControllerRollInput` AxisValue))

(event `InputAxis|Side`
  (params (AxisValue :type "Float (single-precision)"))
  (`self.AddControllerPitchInput` AxisValue))

(event `self.ReceiveTick`
  (params (DeltaSeconds :type "Float (single-precision)"))
  ;[1 1 1] Right Propeller
  (`SceneComponent.K2_AddLocalRotation` (`self.Right`) (`KismetMathLibrary.MakeRotator` (* (`GameplayStatics.GetWorldDeltaSeconds`) (`self.Time`))) false false)
  ;[1 1 1] Left Propeller
  (`SceneComponent.K2_AddLocalRotation` (`self.Left`) (`KismetMathLibrary.MakeRotator` (* (`GameplayStatics.GetWorldDeltaSeconds`) (`self.Time`))) false false))

(fn `UserConstructionScript`)